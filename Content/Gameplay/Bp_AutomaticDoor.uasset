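; Automatic sliding double door that stays locked until the Bp_Timer actor fires its timer-started event.
; Unlocking switches the indicator light materials to gray and green and sets IsOpenable.
; Once openable, overlaps with IsInDoorBox play or reverse a timeline.
; The timeline lerps both door meshes in opposite Y directions from locations cached at BeginPlay.
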(event `self.ReceiveBeginPlay`
  (bind _baselocation (`self.BaseLocation`))
  (`KismetArrayLibrary.Array_Add` _baselocation (`SceneComponent.RelativeLocation` (`self.LeftDoorMesh`)))
  (`KismetArrayLibrary.Array_Add` _baselocation (`SceneComponent.RelativeLocation` (`self.RightDoorMesh`)))
  (bind _returnvalue (`GameplayStatics.GetActorOfClass` "/Game/Gameplay/Timer/Bp_Timer.Bp_Timer_C"))
  (add `/Game/Gameplay/Timer/Bp_Timer.Ev_TimerStarted` _returnvalue (delegate `Ev_TimerStarted_Event_0`)))

(event `Ev_TimerStarted_Event_0`
  (`self.UnlockDoor`))

(event `OpenDoorsMeshs`
  (bind _baselocation (`self.BaseLocation`))
  (bind (_direction _operture) (`Timeline|Timeline_0` :!label _label)
    (:`Update`
      (`self.SetLocationOfMesh` (`self.LeftDoorMesh`) _operture (0.0 -90.0 0.0) (`|GetArrayItem` _baselocation 1))
      (`self.SetLocationOfMesh` (`self.RightDoorMesh`) _operture (0.0 90.0 0.0) (`|GetArrayItem` _baselocation 2)))))

(event `CloseDoorsMeshs`
  (goto _label :!via `Reverse`))

(event `self.IsInDoorBox.OnComponentBeginOverlap`
  (params (OverlappedComponent :type "PrimitiveComponent Object Reference") (OtherActor :type "Actor Object Reference") (OtherComp :type "PrimitiveComponent Object Reference") (OtherBodyIndex :type Integer) (bFromSweep :type Boolean) (SweepResult :type "HitResult Structure (by ref)"))
  (if (`self.IsOpenable`)
    (`self.OpenDoorsMeshs`)))

(event `self.IsInDoorBox.OnComponentEndOverlap`
  (params (OverlappedComponent :type "PrimitiveComponent Object Reference") (OtherActor :type "Actor Object Reference") (OtherComp :type "PrimitiveComponent Object Reference") (OtherBodyIndex :type Integer))
  (if (`self.IsOpenable`)
    (`self.CloseDoorsMeshs`)))

(fn `SetLocationOfMesh`
  (params (self2 :type "SceneComponent Object Reference") (Alpha :type "Float (double-precision)") (Dir :type "Vector Structure") (BaseLocation :type "Vector Structure"))
  (bind _returnvalue (`KismetMathLibrary.Conv_FloatToDouble` 1.0))
  (bind (_x _y _z) (`KismetMathLibrary.BreakVector3f` BaseLocation))
  (bind _returnvalue_2 (`KismetMathLibrary.Lerp` _z (+ _z (* _returnvalue (.z Dir))) Alpha))
  (`KismetSystemLibrary.PrintString` (`KismetStringLibrary.Conv_DoubleToString` _returnvalue_2) true true (struct :`R` 0.99937 :`B` 1.0 :`A` 1.0))
  (`SceneComponent.K2_SetRelativeLocation` self2 (`KismetMathLibrary.MakeVector` (`KismetMathLibrary.Lerp` _x (+ _x (* _returnvalue (.x Dir))) Alpha) (`KismetMathLibrary.Lerp` _y (+ _y (* _returnvalue (.y Dir))) Alpha) _returnvalue_2) false false))

(fn `UnlockDoor`
  (`PrimitiveComponent.SetMaterial` (`self.BadLight`) 0 "/Game/Art/PlaceHolder/M_Gray.M_Gray")
  (`PrimitiveComponent.SetMaterial` (`self.GoodLight`) 0 "/Game/Art/PlaceHolder/M_Green.M_Green")
  (set `self.IsOpenable` true))

(fn `UserConstructionScript`)