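; Interactor component that lets its owning actor interact with nearby objects.
; Interact runs a debug-drawn multi-sphere object trace at a given location and radius against one object type.
; Only the first hit is evaluated: if it implements BPI_Interact, it receives InteractWithMessage with the owner.
; The function returns that actor and whether it can be taken, otherwise false.
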(fn `Interact`
  (params (InteractLocation :type "Vector Structure") (DetectionRadius :type "Float (single-precision)"))
  (returns (ActorInteracted :type "Actor Object Reference") (CanBeTaken :type Boolean))
  (bind (_outhits _returnvalue) (`KismetSystemLibrary.SphereTraceMultiForObjects` :`Start` InteractLocation :`End` InteractLocation :`Radius` DetectionRadius :`ObjectTypes` (`|MakeArray` "ObjectTypeQuery7" :!type "EObjectTypeQuery Enum") :`DrawDebugType` "ForDuration" :`DrawTime` 0.3))
  (if _returnvalue
    (for _array_element _outhits
      (bind (_bblockinghit _binitialoverlap _time _distance _location _impactpoint _normal _impactnormal _physmat _hitactor) (`GameplayStatics.BreakHitResult` _array_element))
      (if (`KismetSystemLibrary.DoesImplementInterface` _hitactor "/Game/Gameplay/InteractionSystem/BPI_Interact.BPI_Interact_C")
        (bind _canbetaken (message `/Game/Gameplay/InteractionSystem/BPI_Interact.InteractWith` _hitactor (`self.GetOwner`)))
        (return _hitactor _canbetaken)
        (else
          (return null false)))))
  (return null false))