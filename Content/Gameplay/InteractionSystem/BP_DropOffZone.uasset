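; Drop-off zone actor for depositing takable items, with a box trigger and a deposit function.
; DropTakable checks IsItemRequired, then either plays a validation sound, broadcasts deposit success with the item's data and destroys it, or plays a denied sound.
; The required-item check is a stub that always passes, pending a checklist test.
; Box overlaps run the IsTakable class check but leave its result unused.
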(event `self.Box.OnComponentBeginOverlap`
  (params (OverlappedComponent :type "PrimitiveComponent Object Reference") (OtherActor :type "Actor Object Reference") (OtherComp :type "PrimitiveComponent Object Reference") (OtherBodyIndex :type Integer) (bFromSweep :type Boolean) (SweepResult :type "HitResult Structure (by ref)"))
  (`self.IsTakable` OtherActor))

(event `self.Box.OnComponentEndOverlap`
  (params (OverlappedComponent :type "PrimitiveComponent Object Reference") (OtherActor :type "Actor Object Reference") (OtherComp :type "PrimitiveComponent Object Reference") (OtherBodyIndex :type Integer))
  (`self.IsTakable` OtherActor))

(fn `DropTakable`
  (params (Takable :type "/Game/Gameplay/InteractionSystem/BP_P_Takable Object Reference"))
  (returns (Success :type Boolean))
  (bind _valid (`self.IsItemRequired` Takable))
  (if _valid
    (`GameplayStatics.PlaySoundAtLocation` "/Game/Sound/Balance/SFX_BalanceValidation.SFX_BalanceValidation" (0.0 0.0 0.0) (struct) 1.0 1.0 0.0 null null null null)
    (`self.Ev_DepositSuccess` (`/Game/Gameplay/InteractionSystem/BP_P_Takable.ItemData` Takable))
    (`self.K2_DestroyActor` Takable)
    (return true)
    (else
      (`GameplayStatics.PlaySoundAtLocation` "/Game/Sound/Balance/SFX_BalanceDenied.SFX_BalanceDenied" (0.0 0.0 0.0) (struct) 1.0 1.0 0.0 null null null null)
      (return false))))

(fn `IsItemRequired`
  (params (TakableTarget :type "/Game/Gameplay/InteractionSystem/BP_P_Takable Object Reference") (NewParam :type Boolean))
  (returns (Valid :type Boolean))
  (return true))

(fn `UserConstructionScript`)