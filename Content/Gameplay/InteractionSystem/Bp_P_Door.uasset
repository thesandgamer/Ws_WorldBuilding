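; Interactable sliding double door that opens through InteractWith, ignoring requests while already open or moving.
; One timeline drives both leaves apart via a lerped relative-location helper, which also debug-prints Z, and reverses to close.
; The IsInDoorBox overlap controls auto-closing: leaving closes an open door, or flags it to close shortly after opening finishes.
; The interaction widget hides during opening and returns once closed.
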(event `self.ReceiveBeginPlay`
  (bind _baselocation (`self.BaseLocation`))
  (bind _asw_ig_display_to_take (`self.GetWidget`))
  (set `/Game/Gameplay/InteractionSystem/W_IG_DisplayToTake.Takable` false _asw_ig_display_to_take)
  (`/Game/Gameplay/InteractionSystem/W_IG_DisplayToTake.Setup` _asw_ig_display_to_take)
  (`self.Show Hide Widget` false)
  (`KismetArrayLibrary.Array_Add` _baselocation (`SceneComponent.RelativeLocation` (`self.LeftDoorMesh`)))
  (`KismetArrayLibrary.Array_Add` _baselocation (`SceneComponent.RelativeLocation` (`self.RightDoorMesh`))))

(event `OpenDoorsMeshs`
  (bind _baselocation (`self.BaseLocation`))
  (`GameplayStatics.PlaySoundAtLocation` "/Game/Sound/Door/SFX_DoorOpen.SFX_DoorOpen" (0.0 0.0 0.0) (struct) 1.0 1.0 0.0 null null null null)
  (`self.Show Hide Widget` false)
  (bind (_direction _operture) (`Timeline|MovingTimeline` :!via `PlayFromStart` :!label _label)
    (:`Update`
      (`self.SetLocationOfMesh` (`self.LeftDoorMesh`) _operture (0.0 -90.0 0.0) (`|GetArrayItem` _baselocation 1))
      (`self.SetLocationOfMesh` (`self.RightDoorMesh`) _operture (0.0 90.0 0.0) (`|GetArrayItem` _baselocation 2)))
    (:`Finished`
      (bind _output_get (set `self.Open` (`|EnumEquality` _direction "Forward")))
      (set `self.Moving` false)
      (`|ExecutionSequence`
        (:`then_0`
          (`KismetSystemLibrary.Delay` 1.0)
          (if (`|EnumEquality` _direction "Forward")
            (if (`self.HaveToClose`)
              (`self.CloseDoorsMeshs`))))
        (:`then_1`
          (if (not _output_get)
            (`self.Show Hide Widget` true)))))))

(event `CloseDoorsMeshs`
  (`GameplayStatics.PlaySoundAtLocation` "/Game/Sound/Door/SFX_DoorClose.SFX_DoorClose" (0.0 0.0 0.0) (struct) 1.0 1.0 0.0 null null null null)
  (goto _label :!via `ReverseFromEnd`))

(event `self.IsInDoorBox.OnComponentEndOverlap`
  (params (OverlappedComponent :type "PrimitiveComponent Object Reference") (OtherActor :type "Actor Object Reference") (OtherComp :type "PrimitiveComponent Object Reference") (OtherBodyIndex :type Integer))
  (set `self.HaveToClose` true)
  (if (`self.Open`)
    (`self.CloseDoorsMeshs`)))

(event `self.IsInDoorBox.OnComponentBeginOverlap`
  (params (OverlappedComponent :type "PrimitiveComponent Object Reference") (OtherActor :type "Actor Object Reference") (OtherComp :type "PrimitiveComponent Object Reference") (OtherBodyIndex :type Integer) (bFromSweep :type Boolean) (SweepResult :type "HitResult Structure (by ref)"))
  (set `self.HaveToClose` false))

(fn `InteractWith`
  (params (WhoInteract :type "Actor Object Reference"))
  (returns (CanBeTaken :type Boolean))
  (`self.OpenDoor`)
  (return false))

(fn `OpenDoor`
  (if (not (or (`self.Open`) (`self.Moving`)))
    (set `self.Moving` true)
    (`self.OpenDoorsMeshs`)))

(fn `SetLocationOfMesh`
  (params (self2 :type "SceneComponent Object Reference") (Alpha :type "Float (double-precision)") (Dir :type "Vector Structure") (BaseLocation :type "Vector Structure"))
  (bind _returnvalue (`KismetMathLibrary.Conv_FloatToDouble` 1.0))
  (bind (_x _y _z) (`KismetMathLibrary.BreakVector3f` BaseLocation))
  (bind _returnvalue_2 (`KismetMathLibrary.Lerp` _z (+ _z (* _returnvalue (.z Dir))) Alpha))
  (`KismetSystemLibrary.PrintString` (`KismetStringLibrary.Conv_DoubleToString` _returnvalue_2) true true (struct :`R` 0.99937 :`B` 1.0 :`A` 1.0))
  (`SceneComponent.K2_SetRelativeLocation` self2 (`KismetMathLibrary.MakeVector` (`KismetMathLibrary.Lerp` _x (+ _x (* _returnvalue (.x Dir))) Alpha) (`KismetMathLibrary.Lerp` _y (+ _y (* _returnvalue (.y Dir))) Alpha) _returnvalue_2) false false))

(fn `UserConstructionScript`
  (`parent.UserConstructionScript`))