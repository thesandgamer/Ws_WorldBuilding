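; Base pickup interactable that can be taken, dropped on the ground or handed to a drop-off zone.
; Taking it turns off detection, disables or relaxes mesh collision, and hides its widget if takable.
; A DropOffDetection overlap tracks the touched BP_DropOffZone.
; Dropping offers it to that zone, then traces down to snap it onto WorldStatic ground, restoring collision and widget only if that succeeds.
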(event `self.ReceiveBeginPlay`
  (bind _asw_ig_display_to_take (`self.GetWidget`))
  (set `/Game/Gameplay/InteractionSystem/W_IG_DisplayToTake.Takable` (`self.CanBeTaken`) _asw_ig_display_to_take)
  (`/Game/Gameplay/InteractionSystem/W_IG_DisplayToTake.Setup` _asw_ig_display_to_take)
  (`self.Show Hide Widget` false))

(event `/Game/Gameplay/InteractionSystem/BPI_Interact.Taken`
  (params (Swap :type Boolean))
  (bind _mesh (`self.Mesh`))
  ;[1 1 1] Taken
  (`PrimitiveComponent.SetCollisionEnabled` (`self.DetectionBox`) "NoCollision")
  (if (`self.HaveCollisionWhenTaken`)
    (`PrimitiveComponent.SetCollisionResponseToChannel` _mesh "ECC_Pawn" "ECR_Ignore")
    (else
      (`PrimitiveComponent.SetCollisionEnabled` _mesh "NoCollision")))
  (if (`self.CanBeTaken`)
    (`self.Show Hide Widget` false)))

(event `self.DropOffDetection.OnComponentBeginOverlap`
  (params (OverlappedComponent :type "PrimitiveComponent Object Reference") (OtherActor :type "Actor Object Reference") (OtherComp :type "PrimitiveComponent Object Reference") (OtherBodyIndex :type Integer) (bFromSweep :type Boolean) (SweepResult :type "HitResult Structure (by ref)"))
  ;[1 1 1] TestDrop
  (bind _castdropoffzone (`self.IsDropOffZone` OtherActor)
    (:`ExecTrue`
      (set `self.TouchingDropOffZone` _castdropoffzone))))

(event `self.DropOffDetection.OnComponentEndOverlap`
  (params (OverlappedComponent :type "PrimitiveComponent Object Reference") (OtherActor :type "Actor Object Reference") (OtherComp :type "PrimitiveComponent Object Reference") (OtherBodyIndex :type Integer))
  ;[1 1 1] TestDrop
  (`self.IsDropOffZone` OtherActor
    (:`ExecTrue`
      (set `self.TouchingDropOffZone` null))))

(fn `AttemptDropOff`
  (returns (Success :type Boolean))
  (if (`KismetSystemLibrary.IsValid` (`self.TouchingDropOffZone`))
    (bind _success (`/Game/Gameplay/InteractionSystem/BP_DropOffZone.DropTakable` (`self.TouchingDropOffZone`) self))
    (if _success
      (return true)
      (else
        _)))
  (return false))

(fn `Dropped`
  (returns (Suceed :type Boolean))
  (bind _mesh (`self.Mesh`))
  (`self.AttemptDropOff`)
  (bind _suceeed (`self.ReplaceOnGround`))
  (if _suceeed
    (bind _detectionbox (`self.DetectionBox`)
      (:`then`
        (`PrimitiveComponent.SetCollisionEnabled` _detectionbox "QueryAndPhysics")
        (if (`self.HaveCollisionWhenTaken`)
          (`PrimitiveComponent.SetCollisionResponseToChannel` _mesh "ECC_Pawn" "ECR_Block")
          (else
            (`PrimitiveComponent.SetCollisionEnabled` _mesh "QueryAndPhysics")))
        (`self.Show Hide Widget` true)
        (return true))
      (:`else`))
    (else
      (return false))))

(fn `InteractWith`
  (params (WhoInteract :type "Actor Object Reference"))
  (returns (CanBeTaken :type Boolean))
  (return (`self.CanBeTaken`)))

(fn `ReplaceOnGround`
  (returns (Suceeed :type Boolean))
  (bind _returnvalue (`self.K2_GetActorLocation`))
  (bind (_outhit _returnvalue_2) (`KismetSystemLibrary.LineTraceSingle` _returnvalue (+ _returnvalue (* (* (`self.GetActorUpVector`) (`KismetMathLibrary.Conv_DoubleToVector` -1.0)) (`KismetMathLibrary.Conv_DoubleToVector` 300.0))) "TraceTypeQuery1"))
  (if _returnvalue_2
    (bind (_bblockinghit _binitialoverlap _time _distance _location _impactpoint _normal _impactnormal _physmat _hitactor _hitcomponent) (`GameplayStatics.BreakHitResult` _outhit))
    (if (`|EnumEquality` (`PrimitiveComponent.GetCollisionObjectType` _hitcomponent) "ECC_WorldStatic")
      (bind (_sweephitresult _returnvalue_3) (`self.K2_SetActorLocation` _location))
      (return _returnvalue_3)
      (else
        _)))
  (return false))

(fn `UserConstructionScript`
  (`parent.UserConstructionScript`))