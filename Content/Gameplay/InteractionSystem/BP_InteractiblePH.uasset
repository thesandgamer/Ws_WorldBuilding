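; BP_InteractiblePH is an interactible object that may be picked up and later dropped.
; Interacting moves its DetectionBox to WorldStatic, makes the mesh ignore pawns or lose collision depending on HaveCollisionWhenTaken, and returns CanBeTaken.
; Dropping restores the custom detection channel and mesh collision, then snaps the actor to the surface below using a short trace along its local down vector.
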(event `/Game/Gameplay/InteractionSystem/BPI_Interact.Dropped`
  (bind _mesh (`self.Mesh`))
  (`PrimitiveComponent.SetCollisionObjectType` (`self.DetectionBox`) "ECC_GameTraceChannel1")
  (if (`self.HaveCollisionWhenTaken`)
    (`PrimitiveComponent.SetCollisionResponseToChannel` _mesh "ECC_Pawn" "ECR_Block")
    (else
      (`PrimitiveComponent.SetCollisionEnabled` _mesh "QueryAndPhysics")))
  (`self.ReplaceOnGround`))

(fn `InteractWith`
  (params (WhoInteract :type "Actor Object Reference"))
  (returns (CanBeTaken :type Boolean))
  (bind _mesh (`self.Mesh`))
  (`PrimitiveComponent.SetCollisionObjectType` (`self.DetectionBox`) "ECC_WorldStatic")
  (if (`self.HaveCollisionWhenTaken`)
    (`PrimitiveComponent.SetCollisionResponseToChannel` _mesh "ECC_Pawn" "ECR_Ignore")
    (else
      (`PrimitiveComponent.SetCollisionEnabled` _mesh "NoCollision")))
  (return (`self.CanBeTaken`)))

(fn `ReplaceOnGround`
  (bind _returnvalue (`self.K2_GetActorLocation`))
  (bind (_outhit _returnvalue_2) (`KismetSystemLibrary.LineTraceSingle` _returnvalue (+ _returnvalue (* (* (`self.GetActorUpVector`) (`KismetMathLibrary.Conv_DoubleToVector` -1.0)) (`KismetMathLibrary.Conv_DoubleToVector` 300.0))) "TraceTypeQuery1"))
  (if _returnvalue_2
    (`self.K2_SetActorLocation` (`.Location` (`GameplayStatics.BreakHitResult` _outhit)))))

(fn `UserConstructionScript`
  (`parent.UserConstructionScript`))