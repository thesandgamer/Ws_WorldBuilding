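; Base interactible actor Blueprint that shows a display-to-take widget when something overlaps its DetectionNear area.
; On BeginPlay it copies CanBeTaken into the W_IG_DisplayToTake widget and hides the widget component.
; DetectionNear begin and end overlaps toggle that widget's visibility, with no check on the overlapping actor.
; InteractWith simply returns CanBeTaken and Dropped returns false, with no further pickup or drop logic.
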(event `self.ReceiveBeginPlay`
  (bind _asw_ig_display_to_take (`self.GetWidget`))
  (set `/Game/Gameplay/InteractionSystem/W_IG_DisplayToTake.Takable` (`self.CanBeTaken`) _asw_ig_display_to_take)
  (`self.Show Hide Widget` false))

(event `self.DetectionNear.OnComponentBeginOverlap`
  (params (OverlappedComponent :type "PrimitiveComponent Object Reference") (OtherActor :type "Actor Object Reference") (OtherComp :type "PrimitiveComponent Object Reference") (OtherBodyIndex :type Integer) (bFromSweep :type Boolean) (SweepResult :type "HitResult Structure (by ref)"))
  (`self.Show Hide Widget` true))

(event `self.DetectionNear.OnComponentEndOverlap`
  (params (OverlappedComponent :type "PrimitiveComponent Object Reference") (OtherActor :type "Actor Object Reference") (OtherComp :type "PrimitiveComponent Object Reference") (OtherBodyIndex :type Integer))
  (`self.Show Hide Widget` false))

(fn `Dropped`
  (returns (Suceed :type Boolean))
  (return false))

(fn `GetWidget`
  (returns (`AsW IG Display to Take` :type "/Game/Gameplay/InteractionSystem/W_IG_DisplayToTake Object Reference"))
  (bind _asw_ig_display_to_take (cast `/Game/Gameplay/InteractionSystem/W_IG_DisplayToTake` (`WidgetComponent.GetWidget` (`self.Widget`))))
  (return _asw_ig_display_to_take))

(fn `InteractWith`
  (params (WhoInteract :type "Actor Object Reference"))
  (returns (CanBeTaken :type Boolean))
  (return (`self.CanBeTaken`)))

(fn `Show Hide Widget`
  (params (Show :type Boolean))
  (`SceneComponent.SetVisibility` (`self.Widget`) Show false)
  (return))

(fn `UserConstructionScript`)