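; BP_InteractionWidget is an interaction prompt that shows a W_IG_DisplayToTake widget when something overlaps its detection sphere.
; On BeginPlay it runs the widget's setup, passes it the configurable action text and hides the widget component.
; DetectionNear overlap events toggle the component's visibility without filtering the overlapping actor.
; The construction script sizes the sphere from a radius variable.
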(event `self.ReceiveBeginPlay`
  (bind _asw_ig_display_to_take (`self.GetWidget`))
  (`/Game/Gameplay/InteractionSystem/W_IG_DisplayToTake.Setup` _asw_ig_display_to_take)
  (`/Game/Gameplay/InteractionSystem/W_IG_DisplayToTake.Change Action text` _asw_ig_display_to_take (`self.ActionText`))
  (`self.Show Hide Widget` false))

(event `self.DetectionNear.OnComponentBeginOverlap`
  (params (OverlappedComponent :type "PrimitiveComponent Object Reference") (OtherActor :type "Actor Object Reference") (OtherComp :type "PrimitiveComponent Object Reference") (OtherBodyIndex :type Integer) (bFromSweep :type Boolean) (SweepResult :type "HitResult Structure (by ref)"))
  (`self.Show Hide Widget` true))

(event `self.DetectionNear.OnComponentEndOverlap`
  (params (OverlappedComponent :type "PrimitiveComponent Object Reference") (OtherActor :type "Actor Object Reference") (OtherComp :type "PrimitiveComponent Object Reference") (OtherBodyIndex :type Integer))
  (`self.Show Hide Widget` false))

(fn `GetWidget`
  (returns (`AsW IG Display to Take` :type "/Game/Gameplay/InteractionSystem/W_IG_DisplayToTake Object Reference"))
  (bind _asw_ig_display_to_take (cast `/Game/Gameplay/InteractionSystem/W_IG_DisplayToTake` (`WidgetComponent.GetWidget` (`self.Widget`))))
  (return _asw_ig_display_to_take))

(fn `Show Hide Widget`
  (params (Show :type Boolean))
  (`SceneComponent.SetVisibility` (`self.Widget`) Show false)
  (return))

(fn `UserConstructionScript`
  (`SphereComponent.SetSphereRadius` (`self.DetectionNear`) (`self.In Sphere Radius`) true))