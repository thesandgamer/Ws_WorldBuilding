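; Deposit item actor that displays a mesh as a levitating object with a scan-glitch look.
; Its Set event copies the main mesh's static mesh onto a second mesh component and scales the main mesh.
; It swaps each material slot on the main mesh to the glitch material and, within that loop, plays a Levitation timeline.
; The timeline moves the main mesh by adding a local offset every update.
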(event `Set`
  (params (Scale :type "Vector Structure"))
  (`StaticMeshComponent.SetStaticMesh` (`self.Mesh1`) (`StaticMeshComponent.StaticMesh` (`self.Mesh`)))
  (`SceneComponent.SetWorldScale3D` (`self.Mesh`) Scale)
  (for (_ _array_index) (`MeshComponent.GetMaterials` (`self.Mesh`))
    ;[1 1 1] Set scan material
    (`PrimitiveComponent.SetMaterial` (`self.Mesh`) _array_index "/Game/VFX/Materials/MAI/Scanner/MAI_ScanGlitch1.MAI_ScanGlitch1")
    ;[1 1 1] Go up down
    (bind (_direction _newtrack_0) (`Timeline|levitation`)
      (:`Update`
        (`SceneComponent.K2_AddLocalOffset` (`self.Mesh`) _newtrack_0 false false)))))

(fn `UserConstructionScript`)