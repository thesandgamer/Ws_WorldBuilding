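; Bp_Timer is a countdown timer actor that creates a W_Timer widget on screen and starts counting down from a configurable minutes-and-seconds maximum at BeginPlay.
; A looping one-second timer decrements the time, updates the widget through timespan conversion, and at zero fires a timer-finished dispatcher and resets.
; It also binds to GS_Main's all-items-deposited event to pause the countdown, and exposes start, pause, play and reset events.
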(event `self.ReceiveBeginPlay`
  (bind _returnvalue (`|CreateWidget` "/Game/Gameplay/Timer/W_Timer.W_Timer_C"))
  (bind _output_get (set `self.TimerWidget` _returnvalue))
  (`UserWidget.AddToViewport` _output_get 0)
  (`self.StartTimer`)
  ;[1 1 1] Pause timer when all items depose
  (bind _asgs_main (cast `/Game/Gameplay/Character/GS_Main` (`GameplayStatics.GetGameState`)))
  (add `/Game/Gameplay/Character/GS_Main.Ev_AllItemsDeposit` _asgs_main (delegate `Ev_AllItemsDeposit_Event_0`)))

(event `Ev_AllItemsDeposit_Event_0`
  ;[1 1 1] Pause timer when all items depose
  (`self.PauseTimer`))

(event `PauseTimer`
  (`KismetSystemLibrary.K2_PauseTimerHandle` (`self.Timer`)))

(event `StartTimer`
  (bind (_countdownmax_min _countdownmax_sec) (break `/Game/Gameplay/Timer/Str_Time` (`self.CountdownMax`)))
  (set `self.CurrentTime` (`KismetMathLibrary.Conv_IntToDouble` (+ (* _countdownmax_min 60) _countdownmax_sec)))
  (`self.SetWidgetTimer`)
  (bind _returnvalue (`KismetSystemLibrary.K2_SetTimerDelegate` (delegate `TimePass`) 1.0 true))
  (set `self.Timer` _returnvalue))

(event `PlayTimer`
  (`KismetSystemLibrary.K2_UnPauseTimerHandle` (`self.Timer`)))

(event `ResetTimer`
  (set `self.CurrentTime` 0.0)
  (`KismetSystemLibrary.K2_ClearAndInvalidateTimerHandle` (`self.Timer`)))

(event `TimePass`
  (bind _currenttime (`self.CurrentTime`))
  (`/Engine/EditorBlueprintResources/StandardMacros.DecrementFloat` _currenttime
    (:`  `
      (`self.SetWidgetTimer`)
      (if (<= _currenttime 0.0)
        (`self.TimerFinished`)))))

(event `TimerFinished`
  (`self.Ev_TimerFinished`)
  (`self.ResetTimer`))

(fn `SetWidgetTimer`
  (bind _timerwidget (`self.TimerWidget`))
  (bind _returnvalue (`KismetMathLibrary.FromSeconds` (`self.CurrentTime`)))
  (`/Game/Gameplay/Timer/W_Timer.SetSec` _timerwidget (`KismetMathLibrary.GetSeconds` _returnvalue))
  (`/Game/Gameplay/Timer/W_Timer.SetMin` _timerwidget (`KismetMathLibrary.GetMinutes` _returnvalue))
  (return))

(fn `UserConstructionScript`)