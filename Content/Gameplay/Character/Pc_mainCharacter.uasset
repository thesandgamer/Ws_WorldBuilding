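; Player controller for the main character that owns the item list UI and creates the dialogue widget.
; On BeginPlay it adds both widgets to the viewport and binds to the character's take and drop item events.
; Those events update each item's taken state in the list, and taking an item also opens the list if closed.
; The ShowList input toggles the list; its show/hide handler is an empty stub.
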(event `self.ReceiveBeginPlay`
  (bind _asch_main_character (`/Game/Editor/FunctionLibrary.GetCharacter`))
  ;[1 1 1] Create List ui
  (bind _returnvalue (`|CreateWidget` "/Game/Gameplay/ItemList/W_ItemListUi.W_ItemListUi_C"))
  (bind _returnvalue_2 (`|CreateWidget` "/Game/Gameplay/DialogueSystem/W_Dialogue.W_Dialogue_C"))
  (bind _output_get (set `self.ItemList` _returnvalue))
  (`UserWidget.AddToViewport` _output_get 0)
  (`UserWidget.AddToViewport` _returnvalue_2 0)
  (add `/Game/Gameplay/ItemList/W_ItemListUi.Ev_ListShowHide` _output_get (delegate `Ev_ListShowHide_Event_0`))
  (add `/Game/Gameplay/Character/Ch_MainCharacter.Ev_TakeItem` _asch_main_character (delegate `Ev_TakeItem_Event_0`))
  (add `/Game/Gameplay/Character/Ch_MainCharacter.Ev_DropItem` _asch_main_character (delegate `Ev_DropItem_Event_0`)))

(event `Ev_DropItem_Event_0`
  (params (ItemData :type "/Game/Gameplay/ItemList/Str_Items Structure"))
  ;[1 1 1] Create List ui
  (`/Game/Gameplay/ItemList/W_ItemListUi.ItemIsTaken` (`self.ItemList`) ItemData false))

(event `Ev_ListShowHide_Event_0`
  (params (Visible :type Boolean))
  ;[1 1 1] Create List ui
)

(event `Ev_TakeItem_Event_0`
  (params (ItemData :type "/Game/Gameplay/ItemList/Str_Items Structure"))
  (bind _itemlist (`self.ItemList`))
  (`/Game/Gameplay/ItemList/W_ItemListUi.ItemIsTaken` _itemlist ItemData true)
  (if (not (`/Game/Gameplay/ItemList/W_ItemListUi.IsOpen` _itemlist))
    (`/Game/Gameplay/ItemList/W_ItemListUi.InteractWithList` _itemlist)))

(event `ShowHideList`
  (`/Game/Gameplay/ItemList/W_ItemListUi.InteractWithList` (`self.ItemList`) :!label _label))

(event `InputAction|ShowList`
  (params (Key :type "Key Structure"))
  (:`Pressed`
    (goto _label)))

(fn `UserConstructionScript`)