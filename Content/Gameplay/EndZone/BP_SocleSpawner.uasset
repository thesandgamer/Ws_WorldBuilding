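; BP_SocleSpawner spawns a pedestal (BP_Socle) in the end zone for each item in GS_Main's ItemsToHave list.
; After a short BeginPlay delay, it steps yaw by 180 over the item count, relative to its own rotation, placing socles at Radius.
; The Ecart variable offsets the index at the list's midpoint to adjust spacing.
; Each socle faces the spawner, receives its item class, and gets a debug sphere.
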(event `self.ReceiveBeginPlay`
  (`KismetSystemLibrary.Delay` 0.2)
  (`self.CreateAllSocles`))

(fn `CreateAllSocles`
  (locals (Index :type Integer))
  (bind _index (`local.Index`))
  (bind _asgs_main (cast `/Game/Gameplay/Character/GS_Main` (`GameplayStatics.GetGameState`)))
  (bind _itemstohave (`/Game/Gameplay/Character/GS_Main.ItemsToHave` _asgs_main))
  (for (_array_element _array_index) _itemstohave
    (bind _returnvalue (`KismetArrayLibrary.Array_Length` _itemstohave))
    (if (== _array_index (/ _returnvalue 2))
      (set `local.Index` (+ _index (`self.Ecart`)))
      (else
        (`/Engine/EditorBlueprintResources/StandardMacros.IncrementInt` _index
          (:`  `
            _))))
    (bind _returnvalue_2 (+ (`self.K2_GetActorLocation`) (* (`KismetMathLibrary.GetForwardVector` (`KismetMathLibrary.ComposeRotators` (`KismetMathLibrary.MakeRotator` 0.0 0.0 (`KismetMathLibrary.Conv_IntToDouble` (* (`local.Index`) (/ 180 _returnvalue)))) (`self.K2_GetActorRotation`))) (`KismetMathLibrary.Conv_DoubleToVector` (`self.Radius`)))))
    (`|SpawnActorFromClass` "/Game/Gameplay/EndZone/BP_Socle.BP_Socle_C" (`KismetMathLibrary.MakeTransform` _returnvalue_2 (`KismetMathLibrary.FindLookAtRotation` _returnvalue_2 (`self.K2_GetActorLocation`))) "Undefined" "OverrideRootScale" null (`.class_5_BE1394934B5D3AC452206EA683EE5002` (break `/Game/Gameplay/ItemList/Str_Items` _array_element)) null)
    (`KismetSystemLibrary.DrawDebugSphere` _returnvalue_2 20.0 12 (struct :`A` 1.0) 50.0 1.0)))

(fn `UserConstructionScript`)